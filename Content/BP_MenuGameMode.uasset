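; Menu game mode that assigns each joining player a default shooter loadout.
; On PostLogin it uses the parity of the PlayerId to alternate rifle and launcher between primary and secondary weapon slots.
; The loadout is stored against the PlayerState through the Loadout subsystem, with a debug print confirming each save.
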(event `self.K2_PostLogin`
  (params (NewPlayer :type "PlayerController Object Reference"))
  (bind _returnvalue (subsystem `LoadoutSubsystem`))
  (bind _playerstate (`Controller.PlayerState` NewPlayer))
  ; 设置数据
  (switch `int` (mod (`PlayerState.PlayerId` _playerstate) 2)
    (:`0`
      (`LoadoutSubsystem.SetLoadoutForPlayerState` _returnvalue _playerstate (make `ShooterLoadout` "/Game/BluePrints/AbilitySystem/Data/weapon/DA_Weapon_Rifle.DA_Weapon_Rifle" "/Game/BluePrints/AbilitySystem/Data/weapon/DA_Weapon_Launcher.DA_Weapon_Launcher"))
      (`KismetSystemLibrary.PrintString` "0存入成功"))
    (:`1`
      (`LoadoutSubsystem.SetLoadoutForPlayerState` _returnvalue _playerstate (make `ShooterLoadout` "/Game/BluePrints/AbilitySystem/Data/weapon/DA_Weapon_Launcher.DA_Weapon_Launcher" "/Game/BluePrints/AbilitySystem/Data/weapon/DA_Weapon_Rifle.DA_Weapon_Rifle"))
      (`KismetSystemLibrary.PrintString` "1存入成功"))))

(event `self.ReceiveBeginPlay`)

(fn `UserConstructionScript`)