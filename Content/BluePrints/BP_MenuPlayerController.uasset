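; Menu player controller that handles primary and secondary weapon selection and starting the match.
; SetSelection stores the chosen index per slot and forwards both to ServerSetLoadout, while GetSelection reads them back.
; ServerSetLoadout validates the indices against WeaponCatalog, saves the loadout for the PlayerState in the loadout subsystem, and prints debug results.
; SeverStartGame_Event runs a ServerTravel console command to the Sandbox map.
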(event `self.ReceiveBeginPlay`)

(event `SeverStartGame_Event`
  (`KismetSystemLibrary.ExecuteConsoleCommand` "ServerTravel /Game/Sandbox" null))

(event `ServerSetLoadout`
  (params (PrimaryIndex :type Integer) (SecondaryIndex :type Integer))
  (bind _returnvalue (`KismetStringLibrary.Conv_IntToString` PrimaryIndex))
  (bind _returnvalue_2 (`KismetStringLibrary.Conv_IntToString` SecondaryIndex))
  (bind _weaponcatalog (`self.WeaponCatalog`))
  (bind _playerstate (`self.PlayerState`))
  (bind _weapons (`ShooterWeaponCatalog.Weapons` _weaponcatalog))
  (bind _output (`|GetArrayItem` _weapons PrimaryIndex))
  (bind _output_2 (`|GetArrayItem` _weapons SecondaryIndex))
  (`/Engine/EditorBlueprintResources/StandardMacros.IsValid` _weaponcatalog
    (:`Is Valid`
      (if (and (`KismetArrayLibrary.Array_IsValidIndex` _weapons PrimaryIndex) (`KismetArrayLibrary.Array_IsValidIndex` _weapons SecondaryIndex))
        (`LoadoutSubsystem.SetLoadoutForPlayerState` (subsystem `LoadoutSubsystem`) _playerstate (make `ShooterLoadout` _output _output_2))
        (`KismetSystemLibrary.PrintString` (`KismetStringLibrary.Concat_StrStr` "服务器收到" (`KismetSystemLibrary.GetDisplayName` _playerstate) "主：" _returnvalue (`KismetSystemLibrary.GetDisplayName` _output) ",副：" _returnvalue_2 (`KismetSystemLibrary.GetDisplayName` _output_2)))
        (else
          (`KismetSystemLibrary.PrintString` (`KismetStringLibrary.Concat_StrStr` "服务器收到非法索引，主：" _returnvalue "副：" _returnvalue_2)))))
    (:`Is Not Valid`
      (`KismetSystemLibrary.PrintString` "WeaponCatalog不存在"))))

(fn `GetSelection`
  (params (Slot :type "EWeaponSlot Enum" :default "Primary"))
  (returns (Selection :type Integer))
  (switch `EWeaponSlot` Slot
    (:`Primary`
      (return (`self.PrimarySelection`)))
    (:`Secondary`
      (return (`self.SecondarySelection`)))))

(fn `SetSelection`
  (params (Slot :type "EWeaponSlot Enum" :default "Primary") (Index :type Integer))
  (switch `EWeaponSlot` Slot
    (:`Primary`
      (bind _output_get (set `self.PrimarySelection` Index)))
    (:`Secondary`
      (bind _output_get_2 (set `self.SecondarySelection` Index))))
  (`KismetSystemLibrary.PrintString` (`KismetStringLibrary.Concat_StrStr` "当前选择，主武器：" (`KismetStringLibrary.Conv_IntToString` (`self.PrimarySelection`)) "副武器：" (`KismetStringLibrary.Conv_IntToString` (`self.SecondarySelection`))))
  (`self.ServerSetLoadout` _output_get _output_get_2))

(fn `UserConstructionScript`)