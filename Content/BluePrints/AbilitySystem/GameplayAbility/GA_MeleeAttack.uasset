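; Melee attack gameplay ability that damages live players near the avatar's combat socket.
; On activation it updates the avatar's facing target to its combat target's location, then plays the attack montage.
; The melee montage event wait begins only from the montage's Completed pin, not in parallel.
; When that event arrives, a radius query around the socket, ignoring the avatar, feeds CauseDamage for each hit, then the ability ends.
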(event `self.K2_ActivateAbility`
  (bind _returnvalue (`self.GetAvatarActorFromActorInfo`))
  (bind _returnvalue_2 (`self.GetAvatarActorFromActorInfo`))
  (bind _returnvalue_3 (message `EnemyInterface.GetCombatTarget` _returnvalue))
  (message `CombatInterface.UpdateFacingTarget` _returnvalue (`Actor.K2_GetActorLocation` _returnvalue_3))
  (`AbilityTask_PlayMontageAndWait.CreatePlayMontageAndWaitProxy` "None" "/Game/QuantumCharacter/Demo/Animations/A_MM_Attack_Montage.A_MM_Attack_Montage"
    (:`OnCompleted`
      (`AbilityTask_WaitGameplayEvent.WaitGameplayEvent` (struct :`TagName` "Event.Montage.Attack.Melee") null
        (:`then`
          (bind _returnvalue_4 (message `CombatInterface.GetCombatSocketLocation` _returnvalue_2))
          (bind _outoverlappingactors (`ShooterAbilitySystemLibrary.GetLivePlayersWithinRadius` _returnvalue_2 (`|MakeArray` _returnvalue_2) 200.0 _returnvalue_4))
          (for _array_element _outoverlappingactors
            (`self.CauseDamage` _array_element))
          (`self.K2_EndAbility`))))))