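; Game mode Blueprint for a KillEmAll mode that assigns each player's weapon loadout to their ShooterPlayerState in PostLogin.
; It applies the loadout the LoadoutSubsystem holds for that player state when the lookup succeeds.
; Otherwise it builds a fallback from the WeaponCatalog's default primary and secondary indices.
; Debug prints report success, fallback, or invalid default indices.
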(event `self.K2_PostLogin`
  (params (NewPlayer :type "PlayerController Object Reference"))
  (bind _playerstate (`Controller.PlayerState` NewPlayer))
  (bind _weapon_catalog (`self.Weapon Catalog`))
  (bind (_outloadout _returnvalue) (`LoadoutSubsystem.GetLoadoutForPlayerState` (subsystem `LoadoutSubsystem`) _playerstate))
  (bind _defaultprimaryindex (`ShooterWeaponCatalog.DefaultPrimaryIndex` _weapon_catalog))
  (bind _defaultsecondaryindex (`ShooterWeaponCatalog.DefaultSecondaryIndex` _weapon_catalog))
  (switch `int` (`KismetMathLibrary.Conv_BoolToInt` _returnvalue)
    (:`0`
      (bind (_outloadout_2 _returnvalue_2) (`ShooterWeaponCatalog.TryMakeLoadout` _weapon_catalog _defaultprimaryindex _defaultsecondaryindex))
      (if _returnvalue_2
        (bind _asshooter_player_state (cast `ShooterPlayerState` _playerstate))
        (`ShooterPlayerState.SetLoadout` _asshooter_player_state _outloadout_2)
        (`KismetSystemLibrary.PrintString` "[兜底]获取失败，走默认")
        (else
          (`KismetSystemLibrary.PrintString` (`KismetStringLibrary.Concat_StrStr` "配置失败，索引值：" (`KismetStringLibrary.Conv_IntToString` _defaultprimaryindex) "，" (`KismetStringLibrary.Conv_IntToString` _defaultsecondaryindex))))))
    (:`1`
      (`KismetSystemLibrary.PrintString` "配置成功")
      (bind _asshooter_player_state_2 (cast `ShooterPlayerState` _playerstate))
      (`ShooterPlayerState.SetLoadout` _asshooter_player_state_2 _outloadout))))

(fn `UserConstructionScript`)